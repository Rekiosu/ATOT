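; Spline-driven wall Blueprint that builds a wall mesh along an editable spline at construction time.
; The construction script calls MiddleMeshSetup, which adds one spline mesh per pair of neighboring spline points, bent by their locations and tangents.
; Start and end cap mesh logic exists but is disconnected, and the computed grid-based section length only feeds unused nodes.
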(fn `MiddleMeshSetup`
  (bind _spline (`self.Spline`))
  (`KismetArrayLibrary.Array_Clear` (`self.Spline Meshs`))
  (set `self.Section Length` (* (.x (`self.GetActorScale3D`)) (`self.GridSize`)))
  (for _index (range (+ (- (`SplineComponent.GetNumberOfSplinePoints` (`self.Spline`)) 2) 1))
    (bind _returnvalue (`AddComponent|NODE_AddSplineMeshComponent-2` :`bManualAttachment` true))
    (`KismetArrayLibrary.Array_Set` (`self.Spline Meshs`) _index _returnvalue true)
    (`StaticMeshComponent.SetStaticMesh` _returnvalue (`self.Wall Mesh Long`))
    (`SplineMeshComponent.SetForwardAxis` _returnvalue "X" true)
    (`SceneComponent.K2_AttachToComponent` _returnvalue (`self.Spline`) "None" "KeepRelative" "KeepRelative" "KeepRelative" true)
    (bind (_location _tangent) (`SplineComponent.GetLocationAndTangentAtSplinePoint` _spline _index "Local"))
    (bind (_location_2 _tangent_2) (`SplineComponent.GetLocationAndTangentAtSplinePoint` _spline (+ _index 1) "Local"))
    (`SplineMeshComponent.SetStartAndEnd` _returnvalue _location _tangent _location_2 _tangent_2 true)))

(fn `UserConstructionScript`
  (`self.MiddleMeshSetup`))