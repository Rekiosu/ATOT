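; City block Blueprint that snaps its instanced buildings, catwalks and tower onto the surface below when Grounded is set.
; The construction script runs GroundStaicMeshInstance on five instanced mesh components, which line-traces each instance down the component's up axis.
; Instances move to the hit location plus an offset, raised only for catwalks, keeping rotation and scale, with no hit check.
; An unconnected event graph loop does the same for child components.
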(event `self.ReceiveBeginPlay`)

(fn `Ground Staic Mesh Instance`
  (params (InstancedStaticMesh :type "InstancedStaticMeshComponent Object Reference") (`Placement Offset` :type "Vector Structure"))
  (for _index (range (`InstancedStaticMeshComponent.GetInstanceCount` InstancedStaticMesh))
    (bind _outinstancetransform (`InstancedStaticMeshComponent.GetInstanceTransform` InstancedStaticMesh _index true))
    (bind _outhit (`KismetSystemLibrary.LineTraceSingle` (.location _outinstancetransform) (+ (.location _outinstancetransform) (* (`SceneComponent.GetUpVector` InstancedStaticMesh) -5000.0)) "TraceTypeQuery1"))
    (`InstancedStaticMeshComponent.UpdateInstanceTransform` InstancedStaticMesh _index (`KismetMathLibrary.MakeTransform` (+ (`.Location` (`GameplayStatics.BreakHitResult` _outhit)) `Placement Offset`) (.rotation _outinstancetransform) (.scale _outinstancetransform)) true false true)))

(fn `UserConstructionScript`
  (if (`self.Grounded?`)
    (`|ExecutionSequence`
      (:`then_0`
        (`self.Ground Staic Mesh Instance` (`self.InstancedStaticMesh_Building1`)))
      (:`then_1`
        (`self.Ground Staic Mesh Instance` (`self.InstancedStaticMesh_Building2`)))
      (:`then_2`
        (`self.Ground Staic Mesh Instance` (`self.InstancedStaticMesh_Building3`)))
      (:`then_3`
        (`self.Ground Staic Mesh Instance` (`self.InstancedStaticMesh_CatWalk1`) (0.0 0.0 1100.0)))
      (:`then_4`
        (`self.Ground Staic Mesh Instance` (`self.InstancedStaticMesh_Tower1`))))))