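; Player character with independent left and right grappling hooks that reel it through the world, with gas particle effects.
; Grapple input spawns a GrappleEnd projectile with an attached cable, and its hook callback flags that side and arms a timed upward-boost gate.
; Each Tick, velocity interpolates toward the hook or both hooks' midpoint and is applied through LaunchCharacter.
; While falling, a radial cable-tension pass also overrides velocity using per-cable length limits.
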(event `/Game/Blueprints/Interfaces/PlayerCharacterInterface.Jump`
  (`self.CharacterJump`))

(event `/Game/Blueprints/Interfaces/PlayerCharacterInterface.LeftGrappleStart`
  (`self.GrappleStart` "NewEnumerator0"))

(event `/Game/Blueprints/Interfaces/PlayerCharacterInterface.RightGrappleStart`
  (`self.GrappleStart` "NewEnumerator1"))

(event `/Game/Blueprints/Interfaces/PlayerCharacterInterface.LeftGrappleStop`
  (`self.GrappleStop` "NewEnumerator0"))

(event `/Game/Blueprints/Interfaces/PlayerCharacterInterface.RightGrappleStop`
  (`self.GrappleStop` "NewEnumerator1"))

(event `/Game/Blueprints/Interfaces/PlayerCharacterInterface.GrappleHookedOnToSomething`
  (params (GrappleHookReference :type "Actor Object Reference") (WhichGrapple :type "/Game/Blueprints/Enum/GrappleSideDirection Enum" :default "NewEnumerator0"))
  (`self.Hooked` GrappleHookReference WhichGrapple))

(event `self.ReceiveTick`
  (params (DeltaSeconds :type "Float (single-precision)"))
  (`self.CalculateAndApplyReelingForce`)
  (`self.Cable Physics Tick Event`))

(event `UpwardForceEvent`
  (`/Engine/EditorBlueprintResources/StandardMacros.Gate` false :!label _label
    (:`Exit`
      (bind _upward_force (`self.UpwardStartForce`)
        (:`Repeat`
          (set `self.ReelForce` _upward_force))
        (:`Complete`
          (`self.DisableUpwardForce`))))))

(event `EnableUpwardForce`
  (`self.CloseNodeforDuration` 0.5
    (:`Finish`
      (set `self.UpwardForceTimer` 2.0)
      (goto _label :!via `Open`))))

(event `DisableUpwardForce`
  (goto _label :!via `Close`))

(event `Cable Physics Tick Event`
  (`/Engine/EditorBlueprintResources/StandardMacros.Gate` false :!label _label_2
    (:`Exit`
      (`self.WhatGrappleIsHooked`
        (:`Left`
          _)
        (:`Right`
          _)
        (:`Both`
          _))
      (`self.ApplyCableTension`))))

(event `CableLimitNotReached`
  (goto _label_2 :!via `Open`))

(event `CableLimitReached`
  (goto _label_2 :!via `Close`))

(fn `ApplyCableTension`
  (if (`NavMovementComponent.IsFalling` (`self.CharacterMovement`))
    (`self.ApplyGrapplePhysicsForce`)))

(fn `CableMaxDistanceChecker`)

(fn `CalculateAndApplyReelingForce`
  (`self.WhatGrappleIsHooked`
    (:`Left`
      _)
    (:`Right`
      _)
    (:`Both`
      _))
  (`|ExecutionSequence`
    (:`then_0`
      (`self.ReelingForceCalculation`
        (:`Finish`
          (`self.GasActivate`))))
    (:`then_1`
      (`self.UpwardForceEvent`))
    (:`then_2`
      (`self.LaunchCharacter` (`self.ReelForce`) true true))))

(fn `CameraSpring`
  (bind _springarm (`self.SpringArm`))
  (bind _targetarmlength (`SpringArmComponent.TargetArmLength` _springarm))
  (bind _returnvalue (`KismetMathLibrary.MapRangeClamped` (`KismetMathLibrary.Abs` (`KismetMathLibrary.VSize` (`self.GetVelocity`))) 0.0 2000.0 100.0 600.0))
  (set `SpringArmComponent.TargetArmLength` (`KismetMathLibrary.FInterpTo` _targetarmlength _returnvalue (`GameplayStatics.GetWorldDeltaSeconds`) (select `bool` (> _targetarmlength _returnvalue) :`false` 3.0 :`true` 1.0 :!type "Float (single-precision)")) _springarm))

(fn `CharacterJump`
  (if (!= (`NavMovementComponent.IsFalling` (`self.CharacterMovement`)) true)
    (`self.LaunchCharacter` (`KismetMathLibrary.MakeVector` 0.0 0.0 (`self.JumpHeight`)))))

(fn `GasActivate`
  (`ActorComponent.Activate` (`self.ParticleSystem`) false))

(fn `GasDeactivate`
  (`ActorComponent.Deactivate` (`self.ParticleSystem`)))

(fn `GrappleStart`
  (params (Direction :type "/Game/Blueprints/Enum/GrappleSideDirection Enum" :default "NewEnumerator0"))
  (locals (HookStartRef :type "BillboardComponent Object Reference") (GrappleMaxSpeed :type "Float (double-precision)" :default 5000.0))
  (bind _returnvalue (`self.GetVelocity`))
  (bind _cableright (`self.CableRight`))
  (bind _cableleft (`self.CableLeft`))
  (bind _returnvalue_2 (`SceneComponent.K2_GetComponentLocation` (`local.HookStartRef`)))
  (bind _returnvalue_3 (`SceneComponent.K2_GetComponentLocation` (`local.HookStartRef`)))
  (switch `/Game/Blueprints/Enum/GrappleSideDirection` Direction
    (:`NewEnumerator0`
      (set `local.HookStartRef` (`self.hookStartPointLeft`))
      (`/Engine/EditorBlueprintResources/StandardMacros.IsValid` (`self.LeftGrappleRef`)
        (:`Is Not Valid`
          (bind (_outhit _returnvalue_4) (`KismetSystemLibrary.LineTraceSingle` _returnvalue_3 (+ _returnvalue_3 (* (`SceneComponent.GetForwardVector` (`self.Camera`)) (`self.GrappleMaxDistance`))) "TraceTypeQuery1"))
          (if _returnvalue_4
            _
            (else
              _))
          (bind _returnvalue_5 (`|SpawnActorFromClass` "/Game/Blueprints/Grapple/GrappleEnd.GrappleEnd_C" (`KismetMathLibrary.MakeTransform` (.location (`KismetMathLibrary.Conv_VectorToTransform` _returnvalue_3)) (`KismetMathLibrary.Conv_VectorToRotator` (`SceneComponent.GetForwardVector` (`self.Camera`))) (0.1 0.1 0.1)) "Undefined" "OverrideRootScale" null _returnvalue (`local.GrappleMaxSpeed`) self "NewEnumerator0" null))
          (set `self.LeftGrappleRef` _returnvalue_5)
          (`SceneComponent.SetVisibility` _cableleft true false)
          (`CableComponent.SetAttachEndTo` _cableleft _returnvalue_5 "None" "None"))))
    (:`NewEnumerator1`
      (set `local.HookStartRef` (`self.hookStartPointRight`))
      (`/Engine/EditorBlueprintResources/StandardMacros.IsValid` (`self.RightGrappleRef`)
        (:`Is Not Valid`
          (bind (_outhit_2 _returnvalue_6) (`KismetSystemLibrary.LineTraceSingle` _returnvalue_2 (+ _returnvalue_2 (* (`SceneComponent.GetForwardVector` (`self.Camera`)) (`self.GrappleMaxDistance`))) "TraceTypeQuery1"))
          (if _returnvalue_6
            _
            (else
              _))
          (bind _returnvalue_7 (`|SpawnActorFromClass` "/Game/Blueprints/Grapple/GrappleEnd.GrappleEnd_C" (`KismetMathLibrary.MakeTransform` (.location (`KismetMathLibrary.Conv_VectorToTransform` _returnvalue_2)) (`KismetMathLibrary.Conv_VectorToRotator` (`SceneComponent.GetForwardVector` (`self.Camera`))) (0.1 0.1 0.1)) "Undefined" "OverrideRootScale" null _returnvalue (`local.GrappleMaxSpeed`) self "NewEnumerator1" null))
          (set `self.RightGrappleRef` _returnvalue_7)
          (`SceneComponent.SetVisibility` _cableright true false)
          (`CableComponent.SetAttachEndTo` _cableright _returnvalue_7 "None" "None"))))))

(fn `GrappleStop`
  (params (Direction :type "/Game/Blueprints/Enum/GrappleSideDirection Enum" :default "NewEnumerator0"))
  (bind _leftgrappleref (`self.LeftGrappleRef`))
  (bind _rightgrappleref (`self.RightGrappleRef`))
  (bind _cableleft (`self.CableLeft`))
  (bind _cableright (`self.CableRight`))
  (switch `/Game/Blueprints/Enum/GrappleSideDirection` Direction
    (:`NewEnumerator0`
      (`/Engine/EditorBlueprintResources/StandardMacros.IsValid` _leftgrappleref
        (:`Is Valid`
          (`self.K2_DestroyActor` _leftgrappleref)
          (set `self.LeftGrappleRef` null)
          (`SceneComponent.SetVisibility` _cableleft false false)
          (`CableComponent.SetAttachEndTo` _cableleft self "None" "None")
          (set `self.Left is Hooked?` false))))
    (:`NewEnumerator1`
      (`/Engine/EditorBlueprintResources/StandardMacros.IsValid` _rightgrappleref
        (:`Is Valid`
          (`self.K2_DestroyActor` _rightgrappleref)
          (set `self.RightGrappleRef` null)
          (`SceneComponent.SetVisibility` _cableright false false)
          (`CableComponent.SetAttachEndTo` _cableright self "None" "None")
          (set `self.Right is Hooked?` false))))))

(fn `Hooked`
  (params (GrappleHooked :type "Actor Object Reference") (GrappleSide :type "/Game/Blueprints/Enum/GrappleSideDirection Enum" :default "NewEnumerator0"))
  (if (or (== GrappleHooked (`self.LeftGrappleRef`)) (== GrappleHooked (`self.RightGrappleRef`)))
    (switch `/Game/Blueprints/Enum/GrappleSideDirection` GrappleSide
      (:`NewEnumerator0`
        (set `self.Left is Hooked?` true))
      (:`NewEnumerator1`
        (set `self.Right is Hooked?` true)))
    (`self.EnableUpwardForce`)))

(fn `LookRight`
  (params (Amount :type "Float (double-precision)"))
  (returns (Empty :type Boolean))
  (`self.AddControllerYawInput` Amount)
  (return false))

(fn `LookUp`
  (params (Amount :type "Float (double-precision)"))
  (returns (Empty :type Boolean))
  (`self.AddControllerPitchInput` (* Amount -1.0))
  (return false))

(fn `MoveForward`
  (params (Amount :type "Float (double-precision)"))
  (returns (Empty :type Boolean))
  (`PawnMovementComponent.AddInputVector` (`self.CharacterMovement`) (* (`KismetMathLibrary.GetForwardVector` (`self.GetControlRotation`)) Amount) false))

(fn `MoveRight`
  (params (Amount :type "Float (double-precision)"))
  (returns (Empty :type Boolean))
  (`PawnMovementComponent.AddInputVector` (`self.CharacterMovement`) (* (`KismetMathLibrary.GetRightVector` (`self.GetControlRotation`)) Amount) false)
  (return false))

(fn `ReelUpdate`
  (if (`NavMovementComponent.IsFalling` (`self.CharacterMovement`))
    _))

(fn `UserConstructionScript`)