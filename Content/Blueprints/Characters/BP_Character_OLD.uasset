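; Older player character Blueprint with basic movement, look, a launch-based jump and independent left and right grappling hooks.
; Starting a grapple spawns a GrappleEnd projectile along the camera's forward vector and attaches that side's visible cable to it.
; Stopping destroys the projectile and hides the cable.
; The line traces' results go unused, and hooking only sets a Hooked flag, so no pull or swing is implemented here.
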(event `/Game/Blueprints/Interfaces/PlayerCharacterInterface.Jump`
  (`self.CharacterJump`))

(event `/Game/Blueprints/Interfaces/PlayerCharacterInterface.LeftGrappleStart`
  (`self.GrappleStart` "NewEnumerator0"))

(event `/Game/Blueprints/Interfaces/PlayerCharacterInterface.RightGrappleStart`
  (`self.GrappleStart` "NewEnumerator1"))

(event `/Game/Blueprints/Interfaces/PlayerCharacterInterface.LeftGrappleStop`
  (`self.GrappleStop` "NewEnumerator0"))

(event `/Game/Blueprints/Interfaces/PlayerCharacterInterface.RightGrappleStop`
  (`self.GrappleStop` "NewEnumerator1"))

(event `/Game/Blueprints/Interfaces/PlayerCharacterInterface.GrappleHookedOnToSomething`
  (params (GrappleHookReference :type "Actor Object Reference") (WhichGrapple :type "/Game/Blueprints/Enum/GrappleSideDirection Enum" :default "NewEnumerator0"))
  (`self.Hooked` GrappleHookReference WhichGrapple))

(event `self.ReceiveTick`
  (params (DeltaSeconds :type "Float (single-precision)")))

(fn `CharacterJump`
  (if (!= (`NavMovementComponent.IsFalling` (`self.CharacterMovement`)) true)
    (`self.LaunchCharacter` (`KismetMathLibrary.MakeVector` 0.0 0.0 (`self.JumpHeight`)))))

(fn `GrappleStart`
  (params (Direction :type "/Game/Blueprints/Enum/GrappleSideDirection Enum" :default "NewEnumerator0"))
  (locals (HookStartRef :type "BillboardComponent Object Reference") (GrappleMaxSpeed :type "Float (double-precision)" :default 2000.0))
  (bind _cableright (`self.CableRight`))
  (bind _cableleft (`self.CableLeft`))
  (bind _returnvalue (`SceneComponent.K2_GetComponentLocation` (`local.HookStartRef`)))
  (bind _returnvalue_2 (`SceneComponent.K2_GetComponentLocation` (`local.HookStartRef`)))
  (switch `/Game/Blueprints/Enum/GrappleSideDirection` Direction
    (:`NewEnumerator0`
      (set `local.HookStartRef` (`self.hookStartPointLeft`))
      (`/Engine/EditorBlueprintResources/StandardMacros.IsValid` (`self.LeftGrappleRef`)
        (:`Is Not Valid`
          (bind (_outhit _returnvalue_3) (`KismetSystemLibrary.LineTraceSingle` _returnvalue_2 (+ _returnvalue_2 (* (`SceneComponent.GetForwardVector` (`self.Camera`)) (`self.GrappleMaxDistance`))) "TraceTypeQuery1"))
          (if _returnvalue_3
            _
            (else
              _))
          (bind _returnvalue_4 (`|SpawnActorFromClass` "/Game/Blueprints/Grapple/GrappleEnd.GrappleEnd_C" (`KismetMathLibrary.MakeTransform` (.location (`KismetMathLibrary.Conv_VectorToTransform` _returnvalue_2)) (`KismetMathLibrary.Conv_VectorToRotator` (`SceneComponent.GetForwardVector` (`self.Camera`))) (0.1 0.1 0.1)) "Undefined" "OverrideRootScale" null (0.0 0.0 0.0) (`local.GrappleMaxSpeed`) self "NewEnumerator0" null))
          (set `self.LeftGrappleRef` _returnvalue_4)
          (`SceneComponent.SetVisibility` _cableleft true false)
          (`CableComponent.SetAttachEndTo` _cableleft _returnvalue_4 "None" "None"))))
    (:`NewEnumerator1`
      (set `local.HookStartRef` (`self.hookStartPointRight`))
      (`/Engine/EditorBlueprintResources/StandardMacros.IsValid` (`self.RightGrappleRef`)
        (:`Is Not Valid`
          (bind (_outhit_2 _returnvalue_5) (`KismetSystemLibrary.LineTraceSingle` _returnvalue (+ _returnvalue (* (`SceneComponent.GetForwardVector` (`self.Camera`)) (`self.GrappleMaxDistance`))) "TraceTypeQuery1"))
          (if _returnvalue_5
            _
            (else
              _))
          (bind _returnvalue_6 (`|SpawnActorFromClass` "/Game/Blueprints/Grapple/GrappleEnd.GrappleEnd_C" (`KismetMathLibrary.MakeTransform` (.location (`KismetMathLibrary.Conv_VectorToTransform` _returnvalue)) (`KismetMathLibrary.Conv_VectorToRotator` (`SceneComponent.GetForwardVector` (`self.Camera`))) (0.1 0.1 0.1)) "Undefined" "OverrideRootScale" null (0.0 0.0 0.0) (`local.GrappleMaxSpeed`) self "NewEnumerator1" null))
          (set `self.RightGrappleRef` _returnvalue_6)
          (`SceneComponent.SetVisibility` _cableright true false)
          (`CableComponent.SetAttachEndTo` _cableright _returnvalue_6 "None" "None"))))))

(fn `GrappleStop`
  (params (Direction :type "/Game/Blueprints/Enum/GrappleSideDirection Enum" :default "NewEnumerator0"))
  (bind _leftgrappleref (`self.LeftGrappleRef`))
  (bind _rightgrappleref (`self.RightGrappleRef`))
  (bind _cableleft (`self.CableLeft`))
  (bind _cableright (`self.CableRight`))
  (switch `/Game/Blueprints/Enum/GrappleSideDirection` Direction
    (:`NewEnumerator0`
      (`/Engine/EditorBlueprintResources/StandardMacros.IsValid` _leftgrappleref
        (:`Is Valid`
          (`self.K2_DestroyActor` _leftgrappleref)
          (set `self.LeftGrappleRef` null)
          (`SceneComponent.SetVisibility` _cableleft false false)
          (`CableComponent.SetAttachEndTo` _cableleft self "None" "None"))))
    (:`NewEnumerator1`
      (`/Engine/EditorBlueprintResources/StandardMacros.IsValid` _rightgrappleref
        (:`Is Valid`
          (`self.K2_DestroyActor` _rightgrappleref)
          (set `self.RightGrappleRef` null)
          (`SceneComponent.SetVisibility` _cableright false false)
          (`CableComponent.SetAttachEndTo` _cableright self "None" "None"))))))

(fn `Hooked`
  (params (GrappleHooked :type "Actor Object Reference") (GrappleSide :type "/Game/Blueprints/Enum/GrappleSideDirection Enum" :default "NewEnumerator0"))
  (set `self.Hooked?` true))

(fn `LookRight`
  (params (Amount :type "Float (double-precision)"))
  (returns (Empty :type Boolean))
  (`self.AddControllerYawInput` Amount)
  (return false))

(fn `LookUp`
  (params (Amount :type "Float (double-precision)"))
  (returns (Empty :type Boolean))
  (`self.AddControllerPitchInput` (* Amount -1.0))
  (return false))

(fn `MoveForward`
  (params (Amount :type "Float (double-precision)"))
  (returns (Empty :type Boolean))
  (`PawnMovementComponent.AddInputVector` (`self.CharacterMovement`) (* (`KismetMathLibrary.GetForwardVector` (`self.GetControlRotation`)) Amount) false))

(fn `MoveRight`
  (params (Amount :type "Float (double-precision)"))
  (returns (Empty :type Boolean))
  (`PawnMovementComponent.AddInputVector` (`self.CharacterMovement`) (* (`KismetMathLibrary.GetRightVector` (`self.GetControlRotation`)) Amount) false)
  (return false))

(fn `UserConstructionScript`)