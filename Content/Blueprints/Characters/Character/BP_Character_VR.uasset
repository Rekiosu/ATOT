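; VR character Blueprint with grappling hooks, whose only active logic here is a Crosshair function that computes aim points for the left and right hooks.
; Line traces from each hook start point place the crosshairs at the hit or trace end, smoothed by lerp during wide-shot grapple.
; Otherwise they snap, and a zero-length sphere trace at their midpoint sets the grapple-test flag before the middle crosshair is placed there.
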(fn `Crosshair`
  (bind _leftcrosshairplacement (`self.LeftCrosshairPlacement`))
  (bind _right_crosshair_placement (`self.Right Crosshair Placement`))
  (bind _returnvalue (/ (+ (`self.LeftCrosshairPlacement`) (`self.Right Crosshair Placement`)) 2.0))
  (if (`self.Wide Shot Grapple Active`)
    (`|ExecutionSequence`
      (:`then_0`
        (bind (_outhit _returnvalue_2) (`KismetSystemLibrary.LineTraceSingle` (`SceneComponent.K2_GetComponentLocation` (`self.hookStartPointLeft`)) (0.0 0.0 0.0) "TraceTypeQuery1"))
        (if _returnvalue_2
          (bind (_bblockinghit _binitialoverlap _time _distance _location _impactpoint _normal _impactnormal _physmat _hitactor _hitcomponent _hitbonename _hititem _faceindex _tracestart _traceend) (`GameplayStatics.BreakHitResult` _outhit))
          (set `self.LeftCrosshairPlacement` (`KismetMathLibrary.VLerp` _leftcrosshairplacement _location 0.5))
          (else
            (set `self.LeftCrosshairPlacement` (`KismetMathLibrary.VLerp` _leftcrosshairplacement _traceend 0.5)))))
      (:`then_1`
        (bind (_outhit_2 _returnvalue_3) (`KismetSystemLibrary.LineTraceSingle` (`SceneComponent.K2_GetComponentLocation` (`self.hookStartPointRight`)) (0.0 0.0 0.0) "TraceTypeQuery1"))
        (if _returnvalue_3
          (bind (_bblockinghit_2 _binitialoverlap_2 _time_2 _distance_2 _location_2 _impactpoint_2 _normal_2 _impactnormal_2 _physmat_2 _hitactor_2 _hitcomponent_2 _hitbonename_2 _hititem_2 _faceindex_2 _tracestart_2 _traceend_2) (`GameplayStatics.BreakHitResult` _outhit_2))
          (set `self.Right Crosshair Placement` (`KismetMathLibrary.VLerp` _right_crosshair_placement _location_2 0.5))
          (else
            (set `self.Right Crosshair Placement` (`KismetMathLibrary.VLerp` _right_crosshair_placement _traceend_2 0.5))))))
    (else
      (`|ExecutionSequence`
        (:`then_0`
          (bind (_outhit_3 _returnvalue_4) (`KismetSystemLibrary.LineTraceSingle` (`SceneComponent.K2_GetComponentLocation` (`self.hookStartPointLeft`)) (0.0 0.0 0.0) "TraceTypeQuery1"))
          (if _returnvalue_4
            (bind (_bblockinghit_3 _binitialoverlap_3 _time_3 _distance_3 _location_3 _impactpoint_3 _normal_3 _impactnormal_3 _physmat_3 _hitactor_3 _hitcomponent_3 _hitbonename_3 _hititem_3 _faceindex_3 _tracestart_3 _traceend_3) (`GameplayStatics.BreakHitResult` _outhit_3))
            (set `self.LeftCrosshairPlacement` _location_3)
            (else
              (set `self.LeftCrosshairPlacement` _traceend_3))))
        (:`then_1`
          (bind (_outhit_4 _returnvalue_5) (`KismetSystemLibrary.LineTraceSingle` (`SceneComponent.K2_GetComponentLocation` (`self.hookStartPointRight`)) (0.0 0.0 0.0) "TraceTypeQuery2"))
          (if _returnvalue_5
            (bind (_bblockinghit_4 _binitialoverlap_4 _time_4 _distance_4 _location_4 _impactpoint_4 _normal_4 _impactnormal_4 _physmat_4 _hitactor_4 _hitcomponent_4 _hitbonename_4 _hititem_4 _faceindex_4 _tracestart_4 _traceend_4) (`GameplayStatics.BreakHitResult` _outhit_4))
            (set `self.Right Crosshair Placement` _location_4)
            (else
              (set `self.Right Crosshair Placement` _traceend_4))))
        (:`then_2`
          (bind (_outhit_5 _returnvalue_6) (`KismetSystemLibrary.SphereTraceSingle` _returnvalue _returnvalue 50.0 "TraceTypeQuery1" true))
          (if _returnvalue_6
            (set `self.CrosshairGrappleTest` true)
            (else
              (set `self.CrosshairGrappleTest` false)))
          (set `self.MiddleCrosshairPlacement` _returnvalue))))))

(fn `UserConstructionScript`
  (`parent.UserConstructionScript`))