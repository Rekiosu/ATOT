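; BP_TitanBase is a base Titan character that sets its scale at construction from a size category ranging from Very Small to Colossal.
; InitSize optionally randomizes the category, then maps the enum to its configurable scale value.
; It applies that value to the capsule's world scale with random variance rolled independently per axis, so proportions can differ between Titans of the same category.
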(fn `InitSize`
  (locals (Size :type "Float (double-precision)"))
  (bind _maxvariance (`self.MaxVariance`))
  (bind _returnvalue (+ (`local.Size`) (`KismetMathLibrary.RandomFloatInRange` (* _maxvariance -1.0) (* _maxvariance 1.0))))
  (if (`self.Randomize Size?`)
    (set `self.TitanSize` (select `int` (`KismetMathLibrary.RandomInteger` (enumcount `/Game/Blueprints/Enum/TitanSizes`)) :`0` "NewEnumerator0" :`1` "NewEnumerator1" :`2` "NewEnumerator2" :`3` "NewEnumerator3" :`4` "NewEnumerator4" :`5` "NewEnumerator5" :!type "/Game/Blueprints/Enum/TitanSizes Enum")))
  (`|ExecutionSequence`
    (:`then_0`
      ;[1 1 1] Set Size Variable based off current Enum size
      (switch `/Game/Blueprints/Enum/TitanSizes` (`self.TitanSize`)
        (:`NewEnumerator0`
          (set `local.Size` (`self.Very Small Size`)))
        (:`NewEnumerator1`
          (set `local.Size` (`self.Small Size`)))
        (:`NewEnumerator2`
          (set `local.Size` (`self.Medium Size`)))
        (:`NewEnumerator3`
          (set `local.Size` (`self.Large Size`)))
        (:`NewEnumerator4`
          (set `local.Size` (`self.Very Large Size`)))
        (:`NewEnumerator5`
          (set `local.Size` (`self.Colossal Size`)))))
    (:`then_1`
      ;[1 1 1] Variance
      (`SceneComponent.SetWorldScale3D` (`self.CapsuleComponent`) (`KismetMathLibrary.MakeVector` _returnvalue _returnvalue _returnvalue)))))

(fn `UserConstructionScript`
  (locals (Sies :type "Float (double-precision)"))
  (`self.InitSize`))