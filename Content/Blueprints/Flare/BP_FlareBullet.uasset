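; BP_FlareBullet is the projectile actor for a fired flare.
; On BeginPlay it spawns a BP_ParticleFlare in its configured flare colour at its own transform and attaches it to itself so the effect follows the bullet.
; After its Life delay it tells the particle actor to deactivate the flare, then destroys itself.
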(event `self.ReceiveBeginPlay`
  (bind (_returnvalue_location _returnvalue_rotation) (`KismetMathLibrary.BreakTransform` (`self.GetTransform`)))
  (bind _returnvalue (`|SpawnActorFromClass` "/Game/Blueprints/Particles/BP_ParticleFlare.BP_ParticleFlare_C" (`KismetMathLibrary.MakeTransform` _returnvalue_location _returnvalue_rotation) "Undefined" "OverrideRootScale" null (`self.Flare Colour`) null))
  (bind _output_get (set `self.ParticleRef` _returnvalue))
  (`self.K2_AttachToActor` _output_get self "None" "SnapToTarget" "SnapToTarget" "KeepRelative" true)
  (`KismetSystemLibrary.Delay` (`self.Life`))
  (`/Game/Blueprints/Particles/BP_ParticleFlare.DeactivateFlare` (`self.ParticleRef`))
  (`self.K2_DestroyActor`))

(fn `UserConstructionScript`)