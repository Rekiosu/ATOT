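; FlareBullet is a flare projectile actor with a colour variant and a limited lifetime.
; The construction script switches on FlareColour to apply the matching red, black, purple, green or yellow flare material to both the sphere mesh and the particle system.
; On BeginPlay it waits for the Life duration, then destroys itself.
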(event `self.ReceiveBeginPlay`
  (`KismetSystemLibrary.Delay` (`self.Life`))
  (`self.K2_DestroyActor`))

(fn `UserConstructionScript`
  (bind _sphere (`self.Sphere`))
  (bind _particlesystem (`self.ParticleSystem`))
  (switch `/Game/Blueprints/Enum/FlareColour` (`self.Flare Colour`)
    (:`NewEnumerator0`
      (`PrimitiveComponent.SetMaterial` _sphere 0 "/Game/Art/Materials/Characters/Flare/M_Flare_Red.M_Flare_Red")
      (`PrimitiveComponent.SetMaterial` _particlesystem 0 "/Game/Art/Materials/Characters/Flare/M_Flare_Red.M_Flare_Red"))
    (:`NewEnumerator1`
      (`PrimitiveComponent.SetMaterial` _sphere 0 "/Game/Art/Materials/Characters/Flare/M_Flare_Black.M_Flare_Black")
      (`PrimitiveComponent.SetMaterial` _particlesystem 0 "/Game/Art/Materials/Characters/Flare/M_Flare_Black.M_Flare_Black"))
    (:`NewEnumerator2`
      (`PrimitiveComponent.SetMaterial` _sphere 0 "/Game/Art/Materials/Characters/Flare/M_Flare_Purple.M_Flare_Purple")
      (`PrimitiveComponent.SetMaterial` _particlesystem 0 "/Game/Art/Materials/Characters/Flare/M_Flare_Purple.M_Flare_Purple"))
    (:`NewEnumerator3`
      (`PrimitiveComponent.SetMaterial` _sphere 0 "/Game/Art/Materials/Characters/Flare/M_Flare_Green.M_Flare_Green")
      (`PrimitiveComponent.SetMaterial` _particlesystem 0 "/Game/Art/Materials/Characters/Flare/M_Flare_Green.M_Flare_Green"))
    (:`NewEnumerator4`
      (`PrimitiveComponent.SetMaterial` _sphere 0 "/Game/Art/Materials/Characters/Flare/M_Flare_Yellow.M_Flare_Yellow")
      (`PrimitiveComponent.SetMaterial` _particlesystem 0 "/Game/Art/Materials/Characters/Flare/M_Flare_Yellow.M_Flare_Yellow"))))