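; GrappleEnd is the projectile actor for the end of a grapple hook.
; When its sphere component hits something, it stops the projectile movement and, if the owning character is valid, notifies that character with a self reference and which grapple it is, plus a debug print.
; Setup nodes for ignoring the owner, max speed and spawn velocity are present but unconnected, so they never run here.
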(event `self.ReceiveBeginPlay`)

(event `self.Sphere1.OnComponentHit`
  (params (HitComponent :type "PrimitiveComponent Object Reference") (OtherActor :type "Actor Object Reference") (OtherComp :type "PrimitiveComponent Object Reference") (NormalImpulse :type "Vector Structure") (Hit :type "HitResult Structure (by ref)"))
  (bind _owningcharacter (`self.OwningCharacter`))
  (`MovementComponent.StopMovementImmediately` (`self.ProjectileMovement`))
  (`/Engine/EditorBlueprintResources/StandardMacros.IsValid` _owningcharacter
    (:`Is Valid`
      (message `/Game/Blueprints/Interfaces/PlayerCharacterInterface.GrappleHookedOnToSomething` _owningcharacter self (`self.WhichGrapple`))
      (`KismetSystemLibrary.PrintString` "HIT SOMETHING"))))

(fn `UserConstructionScript`)