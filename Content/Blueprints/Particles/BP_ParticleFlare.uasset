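; BP_ParticleFlare is a particle flare actor whose color is chosen through the Flare enum.
; The construction script maps that choice (red, black, purple, green or yellow) to a matching material instance on the particle system's first element.
; DeactivateFlare stops the particle system, then destroys the actor after a fixed delay.
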(event `DeactivateFlare`
  (`ActorComponent.Deactivate` (`self.ParticleSystem`))
  (`KismetSystemLibrary.Delay` 10.0)
  (`self.K2_DestroyActor`))

(fn `UserConstructionScript`
  (bind _particlesystem (`self.ParticleSystem`))
  (switch `/Game/Blueprints/Enum/FlareColour` (`self.Flare`)
    (:`NewEnumerator0`
      (`PrimitiveComponent.SetMaterial` _particlesystem 0 "/Game/Art/ML/MI_Particle_flare_red.MI_Particle_flare_red"))
    (:`NewEnumerator1`
      (`PrimitiveComponent.SetMaterial` _particlesystem 0 "/Game/Art/ML/MI_Particle_flare_black.MI_Particle_flare_black"))
    (:`NewEnumerator2`
      (`PrimitiveComponent.SetMaterial` _particlesystem 0 "/Game/Art/ML/MI_Particle_flare_Purple.MI_Particle_flare_Purple"))
    (:`NewEnumerator3`
      (`PrimitiveComponent.SetMaterial` _particlesystem 0 "/Game/Art/ML/MI_Particle_flare_green.MI_Particle_flare_green"))
    (:`NewEnumerator4`
      (`PrimitiveComponent.SetMaterial` _particlesystem 0 "/Game/Art/ML/MI_Particle_flare_Yellow.MI_Particle_flare_Yellow"))))