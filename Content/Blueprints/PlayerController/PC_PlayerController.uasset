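; Player controller that relays movement, look, jump, dual grapple and gas boost input to the controlled pawn.
; It caches the pawn once on BeginPlay and forwards each input as a message call after a validity check.
; Holding GasBoost runs a looping timer that repeatedly sends continuous boost requests, and releasing clears it and sends a stop message.
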(event `self.ReceiveBeginPlay`
  (`self.Check Player and Set`))

(event `InputAxis|MoveFoward`
  (params (AxisValue :type "Float (single-precision)"))
  (bind _currentcontrolledpawn (`self.CurrentControlledPawn`))
  (`/Engine/EditorBlueprintResources/StandardMacros.IsValid` _currentcontrolledpawn
    (:`Is Valid`
      (message `/Game/Blueprints/Interfaces/PlayerCharacterInterface.MoveForward` _currentcontrolledpawn AxisValue))))

(event `InputAxis|MoveRight`
  (params (AxisValue :type "Float (single-precision)"))
  (bind _currentcontrolledpawn (`self.CurrentControlledPawn`))
  (`/Engine/EditorBlueprintResources/StandardMacros.IsValid` _currentcontrolledpawn
    (:`Is Valid`
      (message `/Game/Blueprints/Interfaces/PlayerCharacterInterface.MoveRight` _currentcontrolledpawn AxisValue))))

(event `InputAxis|MouseTurn`
  (params (AxisValue :type "Float (single-precision)"))
  (bind _currentcontrolledpawn (`self.CurrentControlledPawn`))
  (`/Engine/EditorBlueprintResources/StandardMacros.IsValid` _currentcontrolledpawn
    (:`Is Valid`
      (message `/Game/Blueprints/Interfaces/PlayerCharacterInterface.LookRight` _currentcontrolledpawn AxisValue))))

(event `InputAxis|MouseLookUp`
  (params (AxisValue :type "Float (single-precision)"))
  (bind _currentcontrolledpawn (`self.CurrentControlledPawn`))
  (`/Engine/EditorBlueprintResources/StandardMacros.IsValid` _currentcontrolledpawn
    (:`Is Valid`
      (message `/Game/Blueprints/Interfaces/PlayerCharacterInterface.LookUp` _currentcontrolledpawn AxisValue))))

(event `InputAction|Jump`
  (params (Key :type "Key Structure"))
  (bind _currentcontrolledpawn (`self.CurrentControlledPawn`))
  (:`Pressed`
    (`/Engine/EditorBlueprintResources/StandardMacros.IsValid` _currentcontrolledpawn
      (:`Is Valid`
        (message `/Game/Blueprints/Interfaces/PlayerCharacterInterface.Jump` _currentcontrolledpawn)))))

(event `InputAction|LeftGrapple`
  (params (Key :type "Key Structure"))
  (bind _currentcontrolledpawn (`self.CurrentControlledPawn`))
  (:`Pressed`
    (`/Engine/EditorBlueprintResources/StandardMacros.IsValid` _currentcontrolledpawn
      (:`Is Valid`
        (message `/Game/Blueprints/Interfaces/PlayerCharacterInterface.LeftGrappleStart` _currentcontrolledpawn))))
  (:`Released`
    (`/Engine/EditorBlueprintResources/StandardMacros.IsValid` _currentcontrolledpawn
      (:`Is Valid`
        (message `/Game/Blueprints/Interfaces/PlayerCharacterInterface.LeftGrappleStop` _currentcontrolledpawn)))))

(event `InputAction|RightGrapple`
  (params (Key :type "Key Structure"))
  (bind _currentcontrolledpawn (`self.CurrentControlledPawn`))
  (:`Pressed`
    (`/Engine/EditorBlueprintResources/StandardMacros.IsValid` _currentcontrolledpawn
      (:`Is Valid`
        (message `/Game/Blueprints/Interfaces/PlayerCharacterInterface.RightGrappleStart` _currentcontrolledpawn))))
  (:`Released`
    (`/Engine/EditorBlueprintResources/StandardMacros.IsValid` _currentcontrolledpawn
      (:`Is Valid`
        (message `/Game/Blueprints/Interfaces/PlayerCharacterInterface.RightGrappleStop` _currentcontrolledpawn)))))

(event `InputAction|GasBoost`
  (params (Key :type "Key Structure"))
  (bind _currentcontrolledpawn (`self.CurrentControlledPawn`))
  (:`Pressed`
    (bind _returnvalue (`KismetSystemLibrary.K2_SetTimerDelegate` (delegate `BoostRequest`) 0.1 true))
    (set `self.SpacebarLoopTimer` _returnvalue))
  (:`Released`
    (`KismetSystemLibrary.K2_ClearAndInvalidateTimerHandle` (`self.SpacebarLoopTimer`))
    (`/Engine/EditorBlueprintResources/StandardMacros.IsValid` _currentcontrolledpawn
      (:`Is Valid`
        (message `/Game/Blueprints/Interfaces/PlayerCharacterInterface.StopContinuousBoostGas` _currentcontrolledpawn)))))

(event `BoostRequest`
  (bind _currentcontrolledpawn (`self.CurrentControlledPawn`))
  (`/Engine/EditorBlueprintResources/StandardMacros.IsValid` _currentcontrolledpawn
    (:`Is Valid`
      (message `/Game/Blueprints/Interfaces/PlayerCharacterInterface.ContinuousBoostGas` _currentcontrolledpawn))))

(fn `Check Player and Set`
  (bind _returnvalue (`self.K2_GetPawn`))
  (`/Engine/EditorBlueprintResources/StandardMacros.IsValid` _returnvalue
    (:`Is Valid`
      (set `self.CurrentControlledPawn` _returnvalue))))

(fn `UserConstructionScript`)